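; BP_BaseCharacter is a character Blueprint that detects the interactable actor the camera is looking at.
; BeginPlay creates a crosshair widget, and each Tick runs a short Visibility line trace forward from the camera.
; Hits implementing the turnstile or interactive interface become FocusedActor and show the crosshair; otherwise the focus clears and the crosshair is removed from the viewport.
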(event `self.ReceiveTick`
  (params (DeltaSeconds :type "Float (single-precision)"))
  (bind _camera (`self.Camera`))
  (bind _widgetcrosshair (`self.WidgetCrosshair`))
  (bind _returnvalue (`SceneComponent.K2_GetComponentLocation` _camera))
  (bind _returnvalue_2 (`Widget.IsInViewport` _widgetcrosshair))
  (`self.WidgetCrosshair`
    (:`then`
      (bind (_outhit _returnvalue_3) (`KismetSystemLibrary.LineTraceSingle` _returnvalue (+ _returnvalue (* (`SceneComponent.GetForwardVector` _camera) 400.0)) "TraceTypeQuery1"))
      (if _returnvalue_3
        (bind (_bblockinghit _binitialoverlap _time _distance _location _impactpoint _normal _impactnormal _physmat _hitactor) (`GameplayStatics.BreakHitResult` _outhit))
        (if (and (`KismetSystemLibrary.IsValid` _hitactor) (or (`KismetSystemLibrary.DoesImplementInterface` _hitactor "/Script/Testovoe_nomix_vr.UTurnstileInterface") (`KismetSystemLibrary.DoesImplementInterface` _hitactor "/Script/Testovoe_nomix_vr.UInteractiveInterface")))
          (set `self.FocusedActor` _hitactor)
          (if (not _returnvalue_2)
            (`UserWidget.AddToViewport` _widgetcrosshair 0))
          (else
            (set `self.FocusedActor` null :!label _label)
            (if _returnvalue_2
              (`Widget.RemoveFromParent` _widgetcrosshair))))
        (else
          (goto _label))))
    (:`else`)))

(event `self.ReceiveBeginPlay`
  (bind _returnvalue (`|CreateWidget` "/Game/main/widgets/Croshair.Croshair_C"))
  (set `self.WidgetCrosshair` _returnvalue))

(fn `UserConstructionScript`)